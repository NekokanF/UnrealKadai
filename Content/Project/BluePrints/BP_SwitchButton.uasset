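; BP_SwitchButton is a floor-style switch that the player triggers by overlapping its box, animating the button mesh along Z with a timeline.
; When the animation finishes, it opens a valid TargetDoor and marks its event finished, and separately activates a valid TargetBox's InterpToMovement.
; The SetEventFinished override calls its parent, sets the button's relative location to zero and disables the trigger's collision.
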(event `self.Box.OnComponentBeginOverlap`
  (params (OverlappedComponent :type "PrimitiveComponent Object Reference") (OtherActor :type "Actor Object Reference") (OtherComp :type "PrimitiveComponent Object Reference") (OtherBodyIndex :type Integer) (bFromSweep :type Boolean) (SweepResult :type "HitResult Structure (by ref)"))
  (cast `/Game/Project/BluePrints/BP_Player` OtherActor)
  (bind (_direction _openz) (`Timeline|SwitchOn`)
    (:`Update`
      (`SceneComponent.K2_SetRelativeLocation` (`self.STM_Button`) (`KismetMathLibrary.MakeVector` 0.0 0.0 _openz) false false))
    (:`Finished`
      (`|ExecutionSequence`
        (:`then_0`
          (bind _targetdoor (`self.TargetDoor`)
            (:`then`
              (`/Game/Project/BluePrints/BP_Door.OpenDoor` _targetdoor)
              (`self.SetEventFinished`))
            (:`else`)))
        (:`then_1`
          (bind _targetbox (`self.TargetBox`)
            (:`then`
              (`ActorComponent.SetActive` (`/Game/Project/BluePrints/BP_MovingBox.InterpToMovement` _targetbox) true false))
            (:`else`)))))))

(event `self.ReceiveBeginPlay`
  (`parent.ReceiveBeginPlay`))

(fn `SetEventFinished`
  (`parent.SetEventFinished`)
  (`SceneComponent.K2_SetRelativeLocation` (`self.STM_Button`) (0.0 0.0 0.0) false false)
  (`PrimitiveComponent.SetCollisionEnabled` (`self.Box`) "NoCollision"))

(fn `UserConstructionScript`)